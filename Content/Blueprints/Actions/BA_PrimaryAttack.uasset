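; BA_PrimaryAttack is a primary attack action that adds an ammo cost to its parent attack action.
; CanStartAction passes only when the parent check passes and the owner's SSAttributeComponent holds at least SpendAmmo.
; AttackDelayElapsed runs the parent logic, then subtracts SpendAmmo from the character's attribute component, so ammo is spent after the attack delay rather than on start.
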(event EventAttackDelayElapsed
  (params (InCharacter :type Character%20Object%20Reference))
  (|CallParentFunction InCharacter)
  (Class|SSAttributeComponent|ApplyAmmoChange (Actor|GetComponentbyClass InCharacter "/Script/SimpleShooter.SSAttributeComponent") (* (Variables|Default|GetSpendAmmo) -1.0)))

(fn CanStartAction
  (bind _returnvalue (|CallParentFunction))
  (if _returnvalue
    (return (>= (Class|SSAttributeComponent|GetAmmo (Actor|GetComponentbyClass (Components|GetOwner (Class|SSAction|GetOwningComponent)) "/Script/SimpleShooter.SSAttributeComponent")) (Variables|Default|GetSpendAmmo)))
    (else
      (return false))))