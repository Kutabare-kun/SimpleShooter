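; BA_Damage is a one-shot action that applies a health change to the actor that owns its action component.
; On start it finds that owner's SSAttributeComponent and passes the Damage value to ApplyHealthChange as the delta, crediting the instigator.
; It then stops immediately, whether or not the component was found, and stopping removes the action from its action component.
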(event EventStartAction
  (params (InInstigator :type Actor%20Object%20Reference))
  (bind _returnvalue (Class|SSAction|GetOwningComponent))
  (bind _returnvalue_2 (Components|GetOwner _returnvalue))
  (bind _returnvalue_3 (Actor|GetComponentbyClass _returnvalue_2 "/Script/SimpleShooter.SSAttributeComponent"))
  (|CallParentFunction InInstigator)
  (Utilities|IsValid _returnvalue_3
    (:Is%20Valid
      (Class|SSAttributeComponent|ApplyHealthChange _returnvalue_3 InInstigator (Variables|Default|GetDamage))
      (Class|SSAction|StopAction InInstigator))
    (:Is%20Not%20Valid
      (Class|SSAction|StopAction InInstigator))))

(event EventStopAction
  (params (InInstigator :type Actor%20Object%20Reference))
  (|CallParentFunction InInstigator)
  (Class|SSActionComponent|RemoveAction (Class|SSAction|GetOwningComponent) self))